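; Game mode for LeaveMeAlone that runs the countdown game timer.
; On BeginPlay it starts a looping one-second timer that decrements GameTime and broadcasts TimerChange on each tick.
; At zero it clears the timer and also broadcasts TimerOver.
; It binds to the player character's health component OnDeath event so the countdown stops when the player dies.
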(event Custom|Stop%20Timer
  (Utilities|Time|ClearandInvalidateTimerbyHandle (Variables|Default|GetGameTimerHandle)))

(event Custom|Change%20Game%20Time
  (bind _output_get (Variables|Default|SetGame%20Time (- (Variables|Default|GetGame%20Time) 1)))
  (if (== _output_get 0)
    (Utilities|Time|ClearandInvalidateTimerbyHandle (Variables|Default|GetGameTimerHandle))
    (Default|CallTimerChange (Variables|Default|GetGame%20Time))
    (Default|CallTimerOver)
    (else
      (Default|CallTimerChange (Variables|Default|GetGame%20Time)))))

(event EventBeginPlay
  (bind _returnvalue (Utilities|Time|SetTimerbyEvent (delegate Custom|Change%20Game%20Time) 1.0 true))
  (Variables|Default|SetGameTimerHandle _returnvalue)
  (bind _aslmadefault_character (Utilities|Casting|CastToLMADefaultCharacter (Game|Player|GetPlayerPawn 0)))
  (EventDispatchers|BindEventtoOnDeath (Actor|GetComponentbyClass _aslmadefault_character "/Script/LeaveMeAlone.LMAHealthComponent") (delegate Custom|Stop%20Timer)))

(event EventTick
  (params (DeltaSeconds :type Float%20%28single-precision%29)))

(fn ConstructionScript)